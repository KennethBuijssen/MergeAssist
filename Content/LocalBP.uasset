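; LocalBP is a scratch Blueprint that prints debug messages, with no other gameplay effect shown.
; BeginPlay prints a greeting and a label naming the Blueprint as Local.
; Tick shows delta time in red, screen-only for a single frame's duration, then assigns Value to itself and prints "Hello".
; Several leftover nodes, including array add, Value setters and a switch, are disconnected and never run.
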(event `self.ReceiveBeginPlay`
  (`KismetSystemLibrary.PrintString` "Hello, World")
  (`KismetSystemLibrary.PrintString` "Current Blueprint: Local"))

(event `self.ReceiveTick`
  (params (DeltaSeconds :type "Float (single-precision)"))
  (`KismetSystemLibrary.PrintString` (`KismetStringLibrary.Conv_DoubleToString` DeltaSeconds) true false (struct :`R` 1.0 :`G` 0.135354 :`B` 0.145301 :`A` 1.0) DeltaSeconds)
  (set `self.Value` (`self.Value`))
  (`KismetSystemLibrary.PrintString` "Hello"))