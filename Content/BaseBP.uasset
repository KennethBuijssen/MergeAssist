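; BaseBP is a scratch Blueprint with test graphs and no evident gameplay role beyond debug printing.
; BeginPlay prints hello messages, and Tick prints each frame's delta seconds, using that same value as the message duration.
; The event graph and a second test graph hold unconnected leftover nodes that never run.
; The test function and test macro graphs are empty.
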(event `self.ReceiveBeginPlay`
  (`KismetSystemLibrary.PrintString` "Hello, World")
  (`KismetSystemLibrary.PrintString` "Hello")
  (`KismetSystemLibrary.PrintString` "Hello"))

(event `self.ReceiveTick`
  (params (DeltaSeconds :type "Float (single-precision)"))
  (`KismetSystemLibrary.PrintString` (`KismetStringLibrary.Conv_DoubleToString` DeltaSeconds) true true (struct :`G` 0.66 :`B` 1.0 :`A` 1.0) DeltaSeconds))

(fn `TestFunctionGraph`)